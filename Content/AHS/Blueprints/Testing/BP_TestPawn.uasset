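; Test pawn for underwater diving mechanics that adds a temporary main UI widget on BeginPlay.
; Each tick it computes depth from the surface height and drains oxygen while submerged outside the submarine, otherwise refilling it; running out only prints "Dead".
; Left click sphere-traces around the pawn and matches the hit actor's display name for "Speed" or "Tank" to set movement speed or oxygen drain rate.
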(event EventBeginPlay
  (bind _returnvalue (UserInterface|CreateWidget "/Game/AHS/UI/Testing/WBP_Temp_MainUI.WBP_Temp_MainUI_C"))
  (UserInterface|Viewport|AddtoViewport _returnvalue 0))

(event Collision|EventActorBeginOverlap
  (params (OtherActor :type Actor%20Object%20Reference)))

(event EventTick
  (params (DeltaSeconds :type Float%20%28single-precision%29))
  (CallFunction|CurrentDepthUI)
  (CallFunction|OxygenTimer))

(event Input|MouseEvents|LeftMouseButton
  (params (Key :type Key%20Structure :default "None"))
  (bind _returnvalue (Transformation|GetActorLocation))
  (:Pressed
    (bind _outhit (Collision|SphereTraceForObjects _returnvalue _returnvalue 2e+02 (Variables|Default|GetObject%20Types) false 0 "ForDuration"))
    (if (Utilities|String|Contains (Utilities|GetDisplayName (.hitactor _outhit)) "Speed")
      (Variables|/Script/Engine.FloatingPawnMovement|SetMaxSpeed (Variables|Default|GetFloatingPawnMovement) 2e+02)
      (elif (Utilities|String|Contains (Utilities|GetDisplayName (.hitactor _outhit)) "Tank")
        (Variables|Default|SetOxygenDecreaseRate 1.0)))))

(fn ConstructionScript)

(fn CurrentDepthUI
  (Variables|Default|SetCurrent_PlayerDepth (Math|Float|Truncate (* (.z (- (Variables|Default|GetSurface) (Transformation|GetActorLocation))) 0.05))))

(fn OxygenTimer
  (if (< (.z (Transformation|GetActorLocation)) (.z (Variables|Default|GetSurface)))
    (if (Variables|Default|GetbIsInSubmarine)
      ;[0.15 0.15 0.15 0.5] 산소 100 회복, 수중 상태 X
      (Variables|Default|SetbIsUnderwater false)
      (Variables|Default|SetOxygen (Variables|Default|GetMaxOxygen))
      (else
        ;[0.15 0.15 0.15 0.5] 바닷속이라면
        ;;[0.15 0.15 0.15 0.5] 수중 상태 O, 산소 고갈
        (Variables|Default|SetbIsUnderwater true)
        (if (<= (Variables|Default|GetOxygen) 0.0)
          ;;[0.15 0.15 0.15 0.5] 산소 <= 0, 죽음
          (Development|PrintString "Dead")
          (else
            ;;[0.15 0.15 0.15 0.5] 초당 산소 고갈
            (Variables|Default|SetOxygen (- (Variables|Default|GetOxygen) (* (Variables|Default|GetOxygenDecreaseRate) (Utilities|Time|GetWorldDeltaSeconds))))))))
    (else
      ;[0.15 0.15 0.15 0.5] 산소 100, 수중 상태 X
      (Variables|Default|SetbIsUnderwater false)
      (Variables|Default|SetOxygen (Variables|Default|GetMaxOxygen)))))